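; Character Blueprint with a grapple that grabs and drags actors carrying an AC_Grapp component while left mouse is held.
; Pressing spawns a BP_Grapple on the cable end, and a view-directed line trace snaps it to the first valid hit.
; The held object interpolates toward the trace end at the captured hit distance.
; Releasing destroys the grapple and throws the object using its remaining offset to that point as velocity.
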(event `EnhancedInput|/Game/Basic/Input/IA_LeftMouse`
  (params (ActionValue :type Boolean) (ElapsedSeconds :type "Float (double-precision)") (TriggeredSeconds :type "Float (double-precision)") (InputAction :type "InputAction Object Reference" :default "/Game/Basic/Input/IA_LeftMouse.IA_LeftMouse"))
  (bind (_returnvalue _outhit) (`self.Line Trace`))
  (bind (_bblockinghit _binitialoverlap _time _distance _location _impactpoint _normal _impactnormal _physmat _hitactor) (`GameplayStatics.BreakHitResult` _outhit))
  (:`Triggered`
    (`self.Grappled Actor`
      (:`then`
        (`self.Interpolate Grappled Object`))
      (:`else`
        (if (and (`self.bIsGrappleCompleted`) _returnvalue)
          (`/Engine/EditorBlueprintResources/StandardMacros.IsValid` (`self.GetComponentByClass` _hitactor "/Game/Task_07/AC_Grapp.AC_Grapp_C")
            (:`Is Valid`
              (set `self.Grappled Actor` _hitactor)
              (`self.K2_AttachToActor` (`self.Grapple `) _hitactor "None" "SnapToTarget" "KeepWorld" "KeepWorld" true)
              (set `CableComponent.CableLength` 100.0 (`self.Cable`))
              (set `self.Distance` _distance)
              (set `self.bIsGrappleCompleted` false)))))))
  (:`Started`
    (`self.Spawn Grapple`))
  (:`Completed`
    (`self.Grapple Completed`)))

(fn `Grapple Completed`
  (set `CableComponent.EndLocation` (0.0 0.0 0.0) (`self.Cable`))
  (`self.K2_DestroyActor` (`self.Grapple `))
  (set `CableComponent.CableLength` 0.0 (`self.Cable`))
  (set `self.Distance` 2000.0)
  (set `self.bIsGrappleCompleted` true)
  (bind _grappled_actor (`self.Grappled Actor`)
    (:`then`
      (`PrimitiveComponent.SetPhysicsLinearVelocity` (`self.GetComponentByClass` _grappled_actor "/Script/Engine.StaticMeshComponent") (`self.Inertia Velocity`) false "None")
      (set `self.Grappled Actor` null))
    (:`else`)))

(fn `Interpolate Grappled Object`
  (bind (_bblockinghit _binitialoverlap _time _distance _location _impactpoint _normal _impactnormal _physmat _hitactor _hitcomponent _hitbonename _bonename _hititem _elementindex _faceindex _tracestart _traceend) (`GameplayStatics.BreakHitResult` (`.OutHit` (`self.Line Trace`))))
  (bind _returnvalue (`self.K2_GetActorLocation` (`self.Grappled Actor`)))
  (set `self.Inertia Velocity` (- _traceend _returnvalue))
  (`self.K2_SetActorLocation` (`self.Grappled Actor`) (`KismetMathLibrary.VInterpTo` _returnvalue _traceend (`GameplayStatics.GetWorldDeltaSeconds`) 2.0) false false))

(fn `Line Trace`
  (returns (ReturnValue :type Boolean) (OutHit :type "HitResult Structure"))
  (bind (_location _rotation) (`Controller.GetPlayerViewPoint` (`self.GetController`)))
  (bind (_outhit _returnvalue) (`KismetSystemLibrary.LineTraceSingle` :`Start` (`self.K2_GetActorLocation`) :`End` (+ (* (`KismetMathLibrary.GetForwardVector` _rotation) (`self.Distance`)) _location) :`TraceChannel` "TraceTypeQuery1" :`DrawDebugType` "ForOneFrame"))
  (return _returnvalue _outhit))

(fn `Spawn Grapple`
  (bind _returnvalue (`|SpawnActorFromClass` "/Game/Task_07/BP_Grapple.BP_Grapple_C" (`SceneComponent.K2_GetComponentToWorld` (`self.GrapplePoint`)) "Undefined" "MultiplyWithRoot" null null))
  (bind _output_get (set `self.Grapple ` _returnvalue))
  (`CableComponent.SetAttachEndTo` (`self.Cable`) _output_get "None" "None"))

(fn `UserConstructionScript`)