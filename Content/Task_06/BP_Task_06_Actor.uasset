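; BP_Task_06_Actor is a homing actor that chases a target actor referenced by the TargetActor variable.
; Each tick it rotates to face the target's current location using a look-at rotation.
; It also overwrites its ProjectileMovement velocity with that look-at direction at a fixed speed, so it steers instantly toward the target with no gradual turning.
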(event `self.ReceiveTick`
  (params (DeltaSeconds :type "Float (single-precision)"))
  (bind _returnvalue (`KismetMathLibrary.FindLookAtRotation` (`self.K2_GetActorLocation`) (`self.K2_GetActorLocation` (`|ConvertAsset` (`self.Target Actor`)))))
  (`self.K2_SetActorRotation` _returnvalue)
  (set `MovementComponent.Velocity` (* (`KismetMathLibrary.GetForwardVector` _returnvalue) 500.0) (`self.ProjectileMovement`)))

(fn `UserConstructionScript`)