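; Player character for Task 05 that loops along a spline in XY, keeping its own height, and fires physics balls with a predicted landing marker.
; Holding left mouse spawns BP_HitPlace and moves it to the predicted trajectory's end.
; Release launches BP_PhysicBall with that same scene-plus-camera forward velocity; both expire shortly after.
; Acceleration input steps a clamped speed modifier, added to distance each tick alongside DeltaSeconds, making movement frame-rate dependent.
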(event `EnhancedInput|/Game/Basic/Input/IA_LeftMouse`
  (params (ActionValue :type Boolean) (ElapsedSeconds :type "Float (double-precision)") (TriggeredSeconds :type "Float (double-precision)") (InputAction :type "InputAction Object Reference" :default "/Game/Basic/Input/IA_LeftMouse.IA_LeftMouse"))
  ;[0.2177 0.2177 0.2177] Инициаация выстрела и сам выстрел
  (:`Triggered`
    (bind _predictresult (`GameplayStatics.Blueprint_PredictProjectilePath_Advanced` (make `PredictProjectilePathParams` :`StartLocation` (`SceneComponent.K2_GetComponentLocation` (`self.Scene`)) :`LaunchVelocity` (`self.Get Velocity`) :`bTraceWithCollision` true :`ProjectileRadius` 12.0 :`TraceChannel` "ECC_Visibility" :`ActorsToIgnore` (`|MakeArray` self (`self.Hit Place`) :!type "Actor Object Reference") :`SimFrequency` 30.0 :`DrawDebugType` "ForOneFrame")))
    (set `self.Location` (`.Location` (break `PredictProjectilePathPointData` (`.LastTraceDestination` (break `PredictProjectilePathResult` _predictresult)))))
    (bind _hit_place (`self.Hit Place`)
      (:`then`
        (`self.K2_SetActorLocation` _hit_place (`self.Location`) false false))
      (:`else`)))
  (:`Started`
    (`self.Spawn Hit Place`))
  (:`Completed`
    (`self.Make Shot`)))

(event `EnhancedInput|/Game/Basic/Input/IA_Acceleration`
  (params (ActionValue :type "Float (double-precision)") (ElapsedSeconds :type "Float (double-precision)") (TriggeredSeconds :type "Float (double-precision)") (InputAction :type "InputAction Object Reference" :default "/Game/Basic/Input/IA_Acceleration.IA_Acceleration"))
  ;[0.2177 0.2177 0.2177] Увеличение/уменьшение скорости
  (:`Started`
    (set `self.Speed Modifier` (`KismetMathLibrary.FClamp` (+ (`self.Speed Modifier`) (* (`KismetMathLibrary.SignOfFloat` ActionValue) 1.0)) 1.0 (`self.Max Speed`)))))

(event `self.ReceiveTick`
  (params (DeltaSeconds :type "Float (single-precision)"))
  (bind (_returnvalue_x _returnvalue_y _returnvalue_z) (`KismetMathLibrary.BreakVector` (`self.K2_GetActorLocation`)))
  (bind (_returnvalue_x_2 _returnvalue_y_2) (`KismetMathLibrary.BreakVector` (`SplineComponent.GetLocationAtDistanceAlongSpline` (`/Game/Task_05/BP_Trajectory.Spline` (`self.Spline Actor`)) (`self.Distance`) "World")))
  ;[0.2177 0.2177 0.2177] Движение по сплайну
  (set `self.Distance` (+ (`self.Distance`) (+ DeltaSeconds (`self.Speed Modifier`))))
  (`self.K2_SetActorLocation` (`KismetMathLibrary.MakeVector` _returnvalue_x_2 _returnvalue_y_2 _returnvalue_z))
  (if (> (`self.Distance`) (`SplineComponent.GetSplineLength` (`/Game/Task_05/BP_Trajectory.Spline` (`self.Spline Actor`))))
    (set `self.Distance` 0.0)))

(fn `Get Velocity`
  (returns (ReturnValue :type "Vector Structure"))
  (return (* (+ (`KismetMathLibrary.GetForwardVector` (`SceneComponent.K2_GetComponentRotation` (`self.Scene`))) (`SceneComponent.GetForwardVector` (`self.Camera`))) 1000.0)))

(fn `Make Shot`
  (bind _returnvalue (`|SpawnActorFromClass` "/Game/Task_05/BP_PhysicBall.BP_PhysicBall_C" (`SceneComponent.K2_GetComponentToWorld` (`self.Scene`)) "Undefined" "MultiplyWithRoot" null null))
  (`PrimitiveComponent.SetPhysicsLinearVelocity` (`/Game/Task_05/BP_PhysicBall.Sphere` _returnvalue) (`self.Get Velocity`) false "None")
  (`self.SetLifeSpan` (`self.Hit Place`) 2.0)
  (`self.SetLifeSpan` _returnvalue 2.0))

(fn `Spawn Hit Place`
  (bind _returnvalue (`|SpawnActorFromClass` "/Game/Task_05/BP_HitPlace.BP_HitPlace_C" (`KismetMathLibrary.MakeTransform` (`self.Location`)) "Undefined" "MultiplyWithRoot" null null))
  (set `self.Hit Place` _returnvalue))

(fn `UserConstructionScript`)