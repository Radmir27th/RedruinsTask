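; BP_ObjectForReplication is an object with three RepNotify values that reports replication updates on screen, apparently for testing.
; Each OnRep handler prints its value, with Value2 and Value3 using colored, keyed, long-lasting messages and Value1 adding a marker string.
; GetOwner casts the outer object to an Actor and caches it, supplying the world context for printing.
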(fn `Get Owner`
  (returns (Owner :type "Actor Object Reference"))
  (bind _owner (`self.Owner`)
    (:`then`
      (return _owner))
    (:`else`
      (bind _asactor (cast `Actor` (`KismetSystemLibrary.GetOuterObject` self)))
      (bind _output_get (set `self.Owner` _asactor))
      (return _output_get))))

(fn `OnRep_Value1`
  (bind _owner (`self.Get Owner`))
  (`KismetSystemLibrary.PrintString` _owner "123123123123123")
  (`KismetSystemLibrary.PrintString` _owner (`KismetStringLibrary.Conv_BoolToString` (`self.Value1`)) true true (struct :`G` 0.66 :`B` 1.0 :`A` 1.0) 123123.0 "val1"))

(fn `OnRep_Value2`
  (`KismetSystemLibrary.PrintString` (`self.Get Owner`) (`KismetStringLibrary.Conv_DoubleToString` (`self.Value2`)) true true (struct :`R` 1.0 :`G` 0.072616 :`A` 1.0) 123123.0 "val2"))

(fn `OnRep_Value3`
  (`KismetSystemLibrary.PrintString` (`self.Get Owner`) (`KismetStringLibrary.Conv_IntToString` (`self.Value3`)) true true (struct :`G` 1.0 :`B` 0.020357 :`A` 1.0) 123123.0 "val3"))