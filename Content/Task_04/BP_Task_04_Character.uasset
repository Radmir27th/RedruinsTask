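; BP_Task_04_Character is a test character for replicating a runtime-created actor component and a RepObject.
; Client-named events forward to server logic, which adds an AC_Replicate component, waits briefly, then passes it to ReplicateComponentToAll to set Comp.
; A second event chain randomizes RepObject's item name and stack amount.
; Tick prints the object's values and component name, coloring the object text green on server and red on client.
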(event `Create Comp_Server`
  ;[0.1635 0.1635 0.1635] Создание компонента
  (if (`KismetSystemLibrary.IsServer`)
    (bind _returnvalue (`|AddComponentByClass` "/Game/Task_04/AC_Replicate.AC_Replicate_C"))
    (set `self.Comp` _returnvalue)
    (`KismetSystemLibrary.Delay` 1.0)
    (`self.Replicate Component To All` (`self.Comp`))))

(event `Replicate Component To All`
  (params (Comp :type "/Game/Task_04/AC_Replicate Object Reference"))
  ;[0.1635 0.1635 0.1635] Создание компонента
  (set `self.Comp` Comp))

(event `Craete Comp_Client`
  ;[0.1635 0.1635 0.1635] Создание компонента
  (`self.Create Comp_Server`))

(event `Set Random Values`
  (bind _repobject (`self.RepObject`))
  ;[0.1635 0.1635 0.1635] Репликация объекта
  (`Object_Task_4.SetItemName` _repobject (`KismetArrayLibrary.Array_Random` (`self.Item Names`)))
  (`Object_Task_4.SetItemStackAmount` _repobject (`KismetMathLibrary.RandomInteger` 500)))

(event `Set Random Value_Client`
  ;[0.1635 0.1635 0.1635] Репликация объекта
  (`self.Set Random Values`))

(event `self.ReceiveTick`
  (params (DeltaSeconds :type "Float (single-precision)"))
  ;[0.1635 0.1635 0.1635] Вывод значений
  (`self.RepObject`
    (:`then`
      (`KismetSystemLibrary.PrintString` (`KismetStringLibrary.Concat_StrStr` (`KismetStringLibrary.Conv_NameToString` (`Object_Task_4.GetItemName` (`self.RepObject`))) " " (`KismetStringLibrary.Conv_IntToString` (`Object_Task_4.GetItemStackAmount` (`self.RepObject`))) " The object: " (`KismetSystemLibrary.GetDisplayName` (`self.RepObject`))) true true (select `bool` (`KismetSystemLibrary.IsServer`) :`false` (struct :`R` 1.0 :`B` 0.063744 :`A` 1.0) :`true` (struct :`G` 1.0 :`B` 0.041367 :`A` 1.0) :!type "LinearColor Structure") DeltaSeconds)
      (bind _comp (`self.Comp`)
        (:`then`
          (`KismetSystemLibrary.PrintString` (`KismetSystemLibrary.GetDisplayName` _comp) true true (struct :`G` 0.66 :`B` 1.0 :`A` 1.0) DeltaSeconds))
        (:`else`)))
    (:`else`)))

(fn `UserConstructionScript`)