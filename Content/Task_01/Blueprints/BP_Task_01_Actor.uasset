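; BP_Task_01_Actor is an interactable test actor with a sphere mesh, an interaction widget and a marker widget.
; On BeginPlay, when IsWorkDebug is set, it registers itself as owner of its W_Marker widget and keeps that widget ticking offscreen.
; Interact swaps the sphere's material, and Detected shows or hides the WCInteract component.
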(event `self.ReceiveBeginPlay`
  (if (`self.bIsWork_Debug`)
    (bind _asw_marker (cast `/Game/Task_01/Widgets/W_Marker` (`WidgetComponent.GetWidget` (`self.W_Marker`))))
    (bind _output_get (set `self.Marker` _asw_marker))
    (`/Game/Task_01/Widgets/W_Marker.Set Own Interact Actor` _output_get self (`self.bIsWork_Debug`))
    (`WidgetComponent.SetTickWhenOffscreen` (`self.W_Marker`) true)))

(event `/Game/Task_01/Blueprints/BPI_Interaction.Interact`
  (`PrimitiveComponent.SetMaterial` (`self.Sphere`) 0 "/Engine/MapTemplates/Materials/BasicAsset01.BasicAsset01"))

(event `/Game/Task_01/Blueprints/BPI_Interaction.Detected`
  (params (`is Detect` :type Boolean))
  (`SceneComponent.SetHiddenInGame` (`self.WC_Interact`) (not `is Detect`) false))

(fn `UserConstructionScript`)