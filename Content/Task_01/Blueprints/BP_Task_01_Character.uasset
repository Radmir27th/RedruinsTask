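; Player character for Task 01 that detects and interacts with objects implementing BPI_Interaction.
; Capsule overlaps and a per-tick visibility trace, from the actor location toward a point ahead of the controller's viewpoint, set the current interaction object and toggle its detected state.
; A missed trace switches detection off only if that object is not overlapping the character.
; IA_Interact sends the interact message to the stored object.
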(event `self.ReceiveBeginPlay`)

(event `self.Capsule.OnComponentBeginOverlap`
  (params (OverlappedComponent :type "PrimitiveComponent Object Reference") (OtherActor :type "Actor Object Reference") (OtherComp :type "PrimitiveComponent Object Reference") (OtherBodyIndex :type Integer) (bFromSweep :type Boolean) (SweepResult :type "HitResult Structure (by ref)"))
  (if (`KismetSystemLibrary.DoesImplementInterface` OtherActor "/Game/Task_01/Blueprints/BPI_Interaction.BPI_Interaction_C")
    (bind _output_get (set `self.Current Interaction Object` OtherActor))
    (message `/Game/Task_01/Blueprints/BPI_Interaction.Detected` _output_get true)))

(event `self.Capsule.OnComponentEndOverlap`
  (params (OverlappedComponent :type "PrimitiveComponent Object Reference") (OtherActor :type "Actor Object Reference") (OtherComp :type "PrimitiveComponent Object Reference") (OtherBodyIndex :type Integer))
  (if (`KismetSystemLibrary.DoesImplementInterface` OtherActor "/Game/Task_01/Blueprints/BPI_Interaction.BPI_Interaction_C")
    (message `/Game/Task_01/Blueprints/BPI_Interaction.Detected` OtherActor false)))

(event `self.ReceiveTick`
  (params (DeltaSeconds :type "Float (single-precision)"))
  (bind _returnvalue (`self.GetController`))
  (bind (_location _rotation) (`Controller.GetPlayerViewPoint` _returnvalue))
  (`/Engine/EditorBlueprintResources/StandardMacros.IsValid` _returnvalue
    (:`Is Valid`
      (bind (_outhit _returnvalue_2) (`KismetSystemLibrary.LineTraceSingle` (`self.K2_GetActorLocation`) (+ _location (* (`KismetMathLibrary.GetForwardVector` _rotation) 400.0)) "TraceTypeQuery1"))
      (bind (_bblockinghit _binitialoverlap _time _distance _location_2 _impactpoint _normal _impactnormal _physmat _hitactor) (`GameplayStatics.BreakHitResult` _outhit))
      (if (and _returnvalue_2 (`KismetSystemLibrary.DoesImplementInterface` _hitactor "/Game/Task_01/Blueprints/BPI_Interaction.BPI_Interaction_C"))
        (message `/Game/Task_01/Blueprints/BPI_Interaction.Detected` _hitactor true)
        (set `self.Current Interaction Object` _hitactor)
        (else
          (bind _current_interaction_object (`self.Current Interaction Object`)
            (:`then`
              (if (not (`self.IsOverlappingActor` _current_interaction_object self))
                (message `/Game/Task_01/Blueprints/BPI_Interaction.Detected` _current_interaction_object false)))
            (:`else`)))))))

(event `EnhancedInput|/Game/Basic/Input/IA_Interact`
  (params (ActionValue :type Boolean) (ElapsedSeconds :type "Float (double-precision)") (TriggeredSeconds :type "Float (double-precision)") (InputAction :type "InputAction Object Reference" :default "/Game/Basic/Input/IA_Interact.IA_Interact"))
  (:`Triggered`
    (bind _current_interaction_object (`self.Current Interaction Object`)
      (:`then`
        (message `/Game/Task_01/Blueprints/BPI_Interaction.Interact` _current_interaction_object))
      (:`else`))))

(fn `UserConstructionScript`)